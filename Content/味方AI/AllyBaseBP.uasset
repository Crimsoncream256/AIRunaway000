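; Base Blueprint for an allied AI actor that gets healed when hit by a bullet.
; BeginPlay plays a sound at its location and fills HP to MaxHP.
; A Sphere overlap with Bullet_FP_BP adds HP and prints debug messages for healing and full health, without clamping to MaxHP.
; A "SpecialBullet" tag check leading to the same heal is left unconnected and never runs.
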(event `self.Sphere.OnComponentBeginOverlap`
  (params (OverlappedComponent :type "PrimitiveComponent Object Reference") (OtherActor :type "Actor Object Reference") (OtherComp :type "PrimitiveComponent Object Reference") (OtherBodyIndex :type Integer) (bFromSweep :type Boolean) (SweepResult :type "HitResult Structure (by ref)"))
  (cast `/Game/FirstPerson/Blueprints/Bullet_FP_BP` OtherActor)
  (`KismetSystemLibrary.PrintString` "特殊回復")
  (bind _output_get (set `self.HP` (+ (`self.HP`) 1)))
  (if (<= (`self.MaxHP`) _output_get)
    (`KismetSystemLibrary.PrintString` "体力満タン")))

(event `self.ReceiveBeginPlay`
  (`GameplayStatics.PlaySoundAtLocation` "/Game/音いろいろ/キャンセル7.キャンセル7" (`self.K2_GetActorLocation`) (struct) 1.0 1.0 0.0 null null null null)
  (bind _output_get (set `self.MaxHP` 10))
  (set `self.HP` _output_get))

(fn `UserConstructionScript`)