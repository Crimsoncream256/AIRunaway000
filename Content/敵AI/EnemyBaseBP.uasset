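; EnemyBaseBP is an enemy actor with hit points that is destroyed when player bullets deplete its HP.
; BeginPlay fills HP and plays an attenuated static sound at its location.
; Sphere overlaps from Bullet_FP_BP and hits from BP_FirstPersonProjectile share one damage path, each removing one HP despite the overlap's "special damage" debug message.
; Death prints messages, stops Soundaudio and destroys the actor; a SpecialBullet tag check is left unconnected.
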(event `self.Sphere.OnComponentBeginOverlap`
  (params (OverlappedComponent :type "PrimitiveComponent Object Reference") (OtherActor :type "Actor Object Reference") (OtherComp :type "PrimitiveComponent Object Reference") (OtherBodyIndex :type Integer) (bFromSweep :type Boolean) (SweepResult :type "HitResult Structure (by ref)"))
  (cast `/Game/FirstPerson/Blueprints/Bullet_FP_BP` OtherActor)
  (`KismetSystemLibrary.PrintString` "特殊ダメージ")
  (bind _output_get (set `self.HP` (- (`self.HP`) 1) :!label _label))
  (if (<= _output_get 0)
    (`KismetSystemLibrary.PrintString` "行動不能")
    (`GameplayStatics.PlaySoundAtLocation` null (0.0 0.0 0.0) (struct) 1.0 1.0 0.0 null null null null)
    (`KismetSystemLibrary.PrintString` "信号が切断されました")
    (`AudioComponent.Stop` (`self.soundaudio`))
    (`self.K2_DestroyActor`)))

(event `self.Sphere.OnComponentHit`
  (params (HitComponent :type "PrimitiveComponent Object Reference") (OtherActor :type "Actor Object Reference") (OtherComp :type "PrimitiveComponent Object Reference") (NormalImpulse :type "Vector Structure") (Hit :type "HitResult Structure (by ref)"))
  (cast `/Game/FirstPerson/Blueprints/BP_FirstPersonProjectile` OtherActor)
  (`KismetSystemLibrary.PrintString` "ダメージ確認")
  (goto _label))

(event `self.ReceiveBeginPlay`
  (`GameplayStatics.PlaySoundAtLocation` "/Game/音いろいろ/mixkit-glitch-static-1457.mixkit-glitch-static-1457" (`self.K2_GetActorLocation`) (struct) 1.0 1.0 0.0 "/Game/NewSoundAttenuation001.NewSoundAttenuation001" null null null)
  (bind _output_get (set `self.MaxHP` 10))
  (set `self.HP` _output_get))

(fn `UserConstructionScript`)