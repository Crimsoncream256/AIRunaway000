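; Capsule enemy Blueprint that triggers the mission-clear sequence when an actor overlaps it while its HP is 1 or lower.
; BeginPlay runs the parent logic and fills HP from MaxHP; this graph never lowers HP.
; The clearing overlap plays collapse and completion sounds, shows ClearWidget with the mouse cursor, switches to UI-only input and pauses the game.
; Other overlaps only print a debug string.
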(event `self.ReceiveBeginPlay`
  (`parent.ReceiveBeginPlay`)
  (bind _output_get (set `self.MaxHP` 3))
  (set `self.HP` _output_get))

(event `self.ReceiveActorBeginOverlap`
  (params (OtherActor :type "Actor Object Reference"))
  (bind _returnvalue (`GameplayStatics.GetPlayerController` 0))
  (if (<= (`self.HP`) 1)
    (`KismetSystemLibrary.PrintString` "AAAAAAAAAAAAAAAAAAAAAAAAAAAA")
    (`GameplayStatics.PlaySound2D` "/Game/音いろいろ/Collapse01.Collapse01" 1.0 1.0 0.0 null null)
    (`GameplayStatics.PlaySound2D` "/Game/音いろいろ/データ表示3.データ表示3" 1.0 1.0 0.0 null null)
    (`GameplayStatics.PlaySound2D` "/Game/音いろいろ/_1_0__Mission_Complete._1_0__Mission_Complete" 3.0 1.0 0.0 null null)
    (bind _returnvalue_2 (`|CreateWidget` "/Game/ClearWidget.ClearWidget_C"))
    (`UserWidget.AddToViewport` _returnvalue_2 0)
    (set `PlayerController.bShowMouseCursor` true _returnvalue)
    (`WidgetBlueprintLibrary.SetInputMode_UIOnlyEx` _returnvalue null)
    (`GameplayStatics.SetGamePaused` true)
    (else
      (`KismetSystemLibrary.PrintString` "????????????????????"))))

(event `self.ReceiveTick`
  (params (DeltaSeconds :type "Float (single-precision)")))

(fn `UserConstructionScript`
  (`parent.UserConstructionScript`))